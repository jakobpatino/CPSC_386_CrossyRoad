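; Log actor that slides along the world Y axis each Tick, scaled by Moving, Multiplier and SpeedUp.
; It looks up BP_Ground every frame and raises SpeedUp while outside a Y band offset from that actor's Rwf1 and Rwf13 components.
; Past the positive Y limit it wraps back to the negative end, creating a looping lane of movement.
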(event `self.ReceiveTick`
  (params (DeltaSeconds :type "Float (single-precision)"))
  (bind (_returnvalue_x _returnvalue_y _returnvalue_z) (`KismetMathLibrary.BreakVector` (`SceneComponent.K2_GetComponentLocation` (`self.Log`))))
  (bind (_returnvalue_x_2 _returnvalue_y_2) (`KismetMathLibrary.BreakVector` (`SceneComponent.K2_GetComponentLocation` (`self.Log`))))
  (bind (_returnvalue_x_3 _returnvalue_y_3) (`KismetMathLibrary.BreakVector` (`SceneComponent.K2_GetComponentLocation` (`self.Log`))))
  (`SceneComponent.K2_AddWorldOffset` (`self.Log`) (`KismetMathLibrary.MakeVector` 0.0 (* DeltaSeconds (`self.moving`) (`self.multiplier`) (`self.speedUp`))) false false)
  (bind _returnvalue (`GameplayStatics.GetActorOfClass` "/Game/Blueprints/BP_Ground.BP_Ground_C"))
  (bind _returnvalue_2 (`GameplayStatics.GetActorOfClass` "/Game/Blueprints/BP_Ground.BP_Ground_C"))
  (bind (_returnvalue_x_4 _returnvalue_y_4) (`KismetMathLibrary.BreakVector` (`SceneComponent.K2_GetComponentLocation` (`/Game/Blueprints/BP_Ground.Rwf1` _returnvalue))))
  (bind (_returnvalue_x_5 _returnvalue_y_5) (`KismetMathLibrary.BreakVector` (`SceneComponent.K2_GetComponentLocation` (`/Game/Blueprints/BP_Ground.Rwf13` _returnvalue_2))))
  (if (or (> _returnvalue_y_3 (- _returnvalue_y_4 450.0)) (< _returnvalue_y_2 (- _returnvalue_y_5 1000.0)))
    (set `self.speedUp` 1.5)
    (else
      (set `self.speedUp` 1.0)))
  (if (> _returnvalue_y 5000.0)
    (`SceneComponent.K2_SetWorldLocation` (`self.Log`) (`KismetMathLibrary.MakeVector` _returnvalue_x -5000.0 _returnvalue_z) false false)))

(fn `UserConstructionScript`)