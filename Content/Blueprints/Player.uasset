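; Player for a Crossy Road-style chicken hopper, handling grid hops, scoring, coins, death and restart.
; Input release shifts a target position and jumps; Tick interpolates toward it with sweeping, reverting when blocked, and lets logs carry Y.
; The detached camera creeps forward; falling too near it or straying sideways summons an eagle.
; Hits detect logs, lilypads, coins and lethal vehicles, while death branches drive effects and the restart widget.
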(event `self.ReceiveBeginPlay`
  (`SceneComponent.SetAbsolute` (`self.Camera`) true true false)
  (bind _returnvalue (`|CreateWidget` "/Game/Blueprints/UI/WBP_Restart.WBP_Restart_C"))
  (set `self.widget` _returnvalue)
  (bind _returnvalue_2 (`|GenericCreateObject` "/Game/Blueprints/UI/Score.Score_C" (`GameplayStatics.GetPlayerController` 0)))
  (`UserWidget.AddToViewport` _returnvalue_2 0)
  (`GameplayStatics.SpawnSound2D` "/Game/Sounds/car-engine-loop-deep.car-engine-loop-deep" 1.0 1.0 0.0 null))

(event `self.ReceiveTick`
  (params (DeltaSeconds :type "Float (single-precision)"))
  (bind _returnvalue_x (`KismetMathLibrary.BreakVector` (`self.K2_GetActorLocation`)))
  (bind _returnvalue (`GameplayStatics.GetPlayerController` 0))
  (bind (_returnvalue_x_2 _returnvalue_y) (`KismetMathLibrary.BreakVector` (`self.K2_GetActorLocation`)))
  (bind _returnvalue_x_3 (`KismetMathLibrary.BreakVector` (`self.K2_GetActorLocation`)))
  (bind (_returnvalue_x_4 _returnvalue_y_2 _returnvalue_z) (`KismetMathLibrary.BreakVector` (`self.K2_GetActorLocation`)))
  (bind (_returnvalue_x_5 _returnvalue_y_3) (`KismetMathLibrary.BreakVector` (`self.K2_GetActorLocation`)))
  (bind (_returnvalue_x_6 _returnvalue_y_4 _returnvalue_z_2) (`KismetMathLibrary.BreakVector` (`self.K2_GetActorLocation`)))
  (bind (_location_placeholder_x _location_placeholder_y _location_placeholder_z) (`KismetMathLibrary.BreakVector` (`self.Location Placeholder`)))
  (bind _newpos_x (`KismetMathLibrary.BreakVector` (`self.NewPos`)))
  (bind (_returnvalue_x_7 _returnvalue_y_5) (`KismetMathLibrary.BreakVector` (`KismetMathLibrary.VInterpTo_Constant` (`self.Location Placeholder`) (`self.NewPos`) DeltaSeconds 1500.0)))
  (bind _returnvalue_x_8 (`KismetMathLibrary.BreakVector` (`SceneComponent.K2_GetComponentLocation` (`self.Camera`))))
  (bind _returnvalue_x_9 (`KismetMathLibrary.BreakVector` (`SceneComponent.K2_GetComponentLocation` (`self.Chicken`))))
  (bind (_returnvalue_x_10 _returnvalue_y_6 _returnvalue_z_3) (`KismetMathLibrary.BreakVector` (`SceneComponent.K2_GetComponentLocation` (`self.Chicken`))))
  (bind _returnvalue_x_11 (`KismetMathLibrary.BreakVector` (`SceneComponent.K2_GetComponentLocation` (`self.Chicken`))))
  (bind _returnvalue_x_12 (`KismetMathLibrary.BreakVector` (`SceneComponent.K2_GetComponentLocation` (`self.Camera`))))
  (if (`self.OnLog`)
    (set `self.Location Placeholder` (`KismetMathLibrary.MakeVector` _returnvalue_x_7 _returnvalue_y_4 _returnvalue_z_2))
    (else
      (bind _output_get (set `self.Location Placeholder` (`KismetMathLibrary.MakeVector` _returnvalue_x_7 _returnvalue_y_5 _returnvalue_z_2)))))
  (bind (_sweephitresult _returnvalue_2) (`self.K2_SetActorLocation` _output_get true))
  (if (not _returnvalue_2)
    (set `self.NewPos` (`self.LastPos`)))
  (`self.CameraMovement` DeltaSeconds)
  (bind _output_get_2 (set `self.Rotation Placeholder` (`KismetMathLibrary.RInterpTo_Constant` (`self.Rotation Placeholder`) (`self.New Rotation`) DeltaSeconds 600.0)))
  (`self.K2_SetActorRotation` _output_get_2)
  (if (>= _returnvalue_x (`self.Furthest Distance`))
    (set `self.Furthest Distance` _newpos_x))
  (set `/Game/Blueprints/UI/Score.DisplayScore` (/ (`KismetMathLibrary.Round` (`self.Furthest Distance`)) (`KismetMathLibrary.FTrunc` (`self.Move`))) (stale `self.ReceiveBeginPlay` _returnvalue_2))
  (if (`self.dead`)
    (if (`self.carDead`)
      (`SceneComponent.K2_SetWorldLocation` (`self.CapsuleComponent`) (`KismetMathLibrary.MakeVector` (- _returnvalue_x_10 5000.0) _returnvalue_y_6 _returnvalue_z_3) false false :!label _label)
      (`SceneComponent.K2_SetWorldLocation` (`self.DeadFX`) (`KismetMathLibrary.MakeVector` _location_placeholder_x _location_placeholder_y (+ _location_placeholder_z 20.0)) false false)
      (if (< _returnvalue_x_9 _returnvalue_x_8)
        (if (not (`self.restartScreen`))
          (if (== (`KismetMathLibrary.RandomIntegerInRange` 0 1) 0)
            (`GameplayStatics.PlaySound2D` "/Game/Sounds/chickendeath.chickendeath" 1.0 1.0 0.0 null null)
            (else
              (`GameplayStatics.PlaySound2D` "/Game/Sounds/chickendeath2.chickendeath2" 1.0 1.0 0.0 null null)))
          (`UserWidget.AddToViewport` (`self.widget`) 0)
          (`WidgetBlueprintLibrary.SetInputMode_UIOnlyEx` _returnvalue null)
          (set `PlayerController.bShowMouseCursor` true _returnvalue)
          (set `self.restartScreen` true)))
      (elif (`self.water`)
        (if (`self.partFX`)
          (goto _label)
          (else
            (`ParticleSystemComponent.SetTemplate` (`self.DeadFX`) "/Game/Blueprints/SplashEffect/Splash.Splash")
            (`ActorComponent.Activate` (`self.DeadFX`) false)
            (set `self.partFX` true)
            (`GameplayStatics.PlaySound2D` "/Game/Sounds/watersplashlow.watersplashlow" 1.0 1.0 0.0 null null)
            (goto _label)))
        (else
          (bind _returnvalue_3 (`GameplayStatics.GetActorOfClass` "/Game/Blueprints/Eagle.Eagle_C"))
          (bind _returnvalue_x_13 (`KismetMathLibrary.BreakVector` (`self.K2_GetActorLocation` _returnvalue_3)))
          (if (< (- _returnvalue_x_13 _returnvalue_x_11) 25.0)
            (goto _label)))))
    (elif (< (`KismetMathLibrary.Abs` (- _returnvalue_x_3 _returnvalue_x_12)) 450.0)
      (set `self.dead` true :!label _label_2)
      (if (not (`self.eagleExists`))
        (`|SpawnActorFromClass` "/Game/Blueprints/Eagle.Eagle_C" (`KismetMathLibrary.MakeTransform` (`KismetMathLibrary.MakeVector` (+ _returnvalue_x_4 2000.0) _returnvalue_y_2 (+ _returnvalue_z 500.0))) "Undefined" "OverrideRootScale" null null)
        (set `self.eagleExists` true))
      (elif (< _returnvalue_y_3 -1000.0)
        (goto _label_2)
        (elif (> _returnvalue_y 1000.0)
          (goto _label_2))))))

(event `InputAction|Forward`
  (params (Key :type "Key Structure"))
  (bind (_returnvalue_x _returnvalue_y) (`KismetMathLibrary.BreakVector` (`self.K2_GetActorLocation`)))
  (bind _dead (`self.dead`))
  (bind (_newpos_x _newpos_y _newpos_z) (`KismetMathLibrary.BreakVector` (`self.NewPos`)))
  (bind _newpos (`self.NewPos`))
  (bind _chicken (`self.Chicken`))
  (bind _chicken_2 (`self.Chicken`))
  (bind _returnvalue (`NavMovementComponent.IsFalling` (`self.CharacterMovement`)))
  (bind (_returnvalue_x_2 _returnvalue_y_2) (`KismetMathLibrary.BreakVector` (`SceneComponent.K2_GetComponentLocation` _chicken_2)))
  (bind (_returnvalue_x_3 _returnvalue_y_3 _returnvalue_z) (`KismetMathLibrary.BreakVector` (`SceneComponent.K2_GetComponentLocation` _chicken)))
  (:`Pressed`
    (if _dead
      _
      (elif (not _returnvalue)
        (`SceneComponent.K2_SetWorldLocation` _chicken (`KismetMathLibrary.MakeVector` _returnvalue_x_3 _returnvalue_y_3 (+ _returnvalue_z (`self.shiftUp`))) false false :!label _label_3)
        (`SceneComponent.SetWorldScale3D` _chicken (100.0 50.0 100.0)))))
  (:`Released`
    (if _dead
      _
      (elif (not _returnvalue)
        (set `self.New Rotation` (struct))
        (set `self.LastPos` _newpos)
        (set `self.NewPos` (+ _newpos (`KismetMathLibrary.MakeVector` (`self.Move`))))
        (`self.Jump` :!label _label_4)
        (if (`self.OnLog`)
          (set `self.OnLog` false)
          (set `self.NewPos` (`KismetMathLibrary.MakeVector` _newpos_x (* (`KismetMathLibrary.Round` (/ _returnvalue_y 300.0)) 300.0) _newpos_z)))
        (`SceneComponent.SetWorldScale3D` _chicken_2 (100.0 100.0 100.0) :!label _label_5)
        (`SceneComponent.K2_SetWorldLocation` _chicken_2 (`KismetMathLibrary.MakeVector` _returnvalue_x_2 _returnvalue_y_2 -70.0) false false)
        (`GameplayStatics.PlaySound2D` "/Game/Sounds/hop2b.hop2b" 1.0 1.0 0.0 null null)
        (`GameplayStatics.PlaySound2D` (select `int` (`KismetMathLibrary.RandomIntegerInRange` 0 35) :`0` "/Game/Sounds/buck1.buck1" :`1` "/Game/Sounds/buck2.buck2" :`2` "/Game/Sounds/buck3.buck3" :`3` "/Game/Sounds/buck4.buck4" :`4` "/Game/Sounds/buck5.buck5" :`5` "/Game/Sounds/buck6.buck6" :`6` "/Game/Sounds/buck7.buck7" :`7` "/Game/Sounds/buck8.buck8" :`8` "/Game/Sounds/buck9.buck9" :`9` "/Game/Sounds/buck10.buck10" :`10` "/Game/Sounds/buck11.buck11" :`11` "/Game/Sounds/buck12.buck12" :!type "SoundBase Object Reference") 1.0 1.0 0.0 null null)))))

(event `InputAction|Back`
  (params (Key :type "Key Structure"))
  (bind _dead (`self.dead`))
  (bind _newpos (`self.NewPos`))
  (bind _returnvalue (`NavMovementComponent.IsFalling` (`self.CharacterMovement`)))
  (:`Pressed`
    (if _dead
      _
      (elif (not _returnvalue)
        (goto _label_3))))
  (:`Released`
    (if _dead
      _
      (elif (not _returnvalue)
        (set `self.New Rotation` (struct :`Yaw` 180.0))
        (set `self.LastPos` _newpos)
        (set `self.NewPos` (+ _newpos (`KismetMathLibrary.MakeVector` (* (`self.Move`) -1.0))))
        (goto _label_4)))))

(event `InputAction|Left`
  (params (Key :type "Key Structure"))
  (bind _dead (`self.dead`))
  (bind _newpos (`self.NewPos`))
  (bind _returnvalue (`NavMovementComponent.IsFalling` (`self.CharacterMovement`)))
  (:`Pressed`
    (if _dead
      _
      (elif (not _returnvalue)
        (goto _label_3))))
  (:`Released`
    (if _dead
      _
      (elif (not _returnvalue)
        (set `self.New Rotation` (struct :`Yaw` 270.0))
        (set `self.LastPos` _newpos)
        (set `self.NewPos` (+ _newpos (`KismetMathLibrary.MakeVector` 0.0 (* (`self.Move`) -1.0))))
        (`self.Jump` :!label _label_6)
        (if (`self.OnLog`)
          (set `self.OnLog` false)
          (goto _label_5)
          (else
            (goto _label_5)))))))

(event `InputAction|Right`
  (params (Key :type "Key Structure"))
  (bind _dead (`self.dead`))
  (bind _newpos (`self.NewPos`))
  (bind _returnvalue (`NavMovementComponent.IsFalling` (`self.CharacterMovement`)))
  (:`Pressed`
    (if _dead
      _
      (elif (not _returnvalue)
        (goto _label_3))))
  (:`Released`
    (if _dead
      _
      (elif (not _returnvalue)
        (set `self.New Rotation` (struct :`Yaw` 90.0))
        (set `self.LastPos` _newpos)
        (set `self.NewPos` (+ _newpos (`KismetMathLibrary.MakeVector` 0.0 (`self.Move`))))
        (goto _label_6)))))

(event `self.ReceiveHit`
  (params (MyComp :type "PrimitiveComponent Object Reference") (Other :type "Actor Object Reference") (OtherComp :type "PrimitiveComponent Object Reference") (bSelfMoved :type Boolean) (HitLocation :type "Vector Structure") (HitNormal :type "Vector Structure") (NormalImpulse :type "Vector Structure") (Hit :type "HitResult Structure (by ref)"))
  (cast `/Game/Blueprints/log` Other
    (:`then`
      (set `self.OnLog` true :!label _label_7)
      (if (== (`KismetMathLibrary.RandomIntegerInRange` 0 1) 0)
        (`GameplayStatics.PlaySound2D` "/Game/Sounds/logjump3.logjump3" 1.0 1.0 0.0 null null)
        (else
          (`GameplayStatics.PlaySound2D` "/Game/Sounds/logjump4.logjump4" 1.0 1.0 0.0 null null))))
    (:`CastFailed`
      (cast `/Game/Blueprints/lillypad` Other
        (:`then`
          (set `self.OnLog` true)
          (`GameplayStatics.PlaySound2D` "/Game/Sounds/lilysplash.lilysplash" 1.0 1.0 0.0 null null))
        (:`CastFailed`
          (cast `/Game/Blueprints/log2` Other
            (:`then`
              (goto _label_7))
            (:`CastFailed`
              (cast `/Game/Blueprints/car` Other
                (:`then`
                  (set `self.dead` true)
                  (set `self.carDead` true)
                  (`GameplayStatics.PlaySound2D` "/Game/Sounds/carhit.carhit" 1.0 1.0 0.0 null null)
                  (`ActorComponent.Activate` (`self.DeadFX`) false :!label _label_8))
                (:`CastFailed`
                  (cast `/Game/Blueprints/car2` Other
                    (:`then`
                      (set `self.dead` true)
                      (set `self.carDead` true)
                      (`GameplayStatics.PlaySound2D` "/Game/Sounds/carhit.carhit" 1.0 1.0 0.0 null null)
                      (goto _label_8))
                    (:`CastFailed`
                      (cast `/Game/Blueprints/truck` Other
                        (:`then`
                          (set `self.dead` true)
                          (set `self.carDead` true)
                          (`GameplayStatics.PlaySound2D` "/Game/Sounds/carhit.carhit" 1.0 1.0 0.0 null null)
                          (goto _label_8))
                        (:`CastFailed`
                          (cast `/Game/Blueprints/truck2` Other
                            (:`then`
                              (set `self.dead` true)
                              (set `self.carDead` true)
                              (`GameplayStatics.PlaySound2D` "/Game/Sounds/carhit.carhit" 1.0 1.0 0.0 null null)
                              (goto _label_8))
                            (:`CastFailed`
                              (cast `/Game/Blueprints/train` Other
                                (:`then`
                                  (set `self.dead` true)
                                  (set `self.carDead` true)
                                  (`GameplayStatics.PlaySound2D` "/Game/Sounds/trainsplat.trainsplat" 1.0 1.0 0.0 null null)
                                  (goto _label_8))
                                (:`CastFailed`
                                  (cast `/Game/Blueprints/train2` Other
                                    (:`then`
                                      (set `self.dead` true)
                                      (set `self.carDead` true)
                                      (`GameplayStatics.PlaySound2D` "/Game/Sounds/trainsplat.trainsplat" 1.0 1.0 0.0 null null)
                                      (goto _label_8))
                                    (:`CastFailed`
                                      (bind _ascoin (cast `/Game/Blueprints/coin` Other))
                                      (`self.K2_DestroyActor` _ascoin)
                                      (bind _result (`/Engine/EditorBlueprintResources/StandardMacros.IncrementInt` (`/Game/Blueprints/UI/Score.Coins` (stale `self.ReceiveBeginPlay` _returnvalue_2)))
                                        (:`  `
                                          (set `/Game/Blueprints/UI/Score.Coins` _result (stale `self.ReceiveBeginPlay` _returnvalue_2))
                                          (`GameplayStatics.PlaySound2D` "/Game/Sounds/Earn_Points.Earn_Points" 1.0 1.0 0.0 null null))))))))))))))))))))))

(fn `CameraMovement`
  (params (DeltaSeconds :type "Float (double-precision)"))
  (bind _returnvalue_x (`KismetMathLibrary.BreakVector` (`self.K2_GetActorLocation`)))
  (bind _camera (`self.Camera`))
  (bind _returnvalue_x_2 (`KismetMathLibrary.BreakVector` (`SceneComponent.K2_GetComponentLocation` (`self.Camera`))))
  (bind (_returnvalue_x_3 _returnvalue_y) (`KismetMathLibrary.BreakVector` (`SceneComponent.K2_GetComponentLocation` _camera)))
  (`SceneComponent.K2_AddLocalOffset` _camera (`KismetMathLibrary.MakeVector` (* (`KismetMathLibrary.Abs` (- _returnvalue_x_2 _returnvalue_x)) DeltaSeconds 0.2)) false false)
  (`SceneComponent.K2_SetWorldLocation` _camera (`KismetMathLibrary.MakeVector` _returnvalue_x_3 _returnvalue_y 1000.0) false false))

(fn `UserConstructionScript`)