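; Truck Blueprint that drives a truck continuously along the world Y axis in an endless loop.
; Each Tick offsets the Truck component in Y by Moving and Multiplier, scaled by delta time for frame-rate independence.
; Once it passes the upper Y limit, it teleports back to the negative end, keeping its X and Z position.
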(event `self.ReceiveTick`
  (params (DeltaSeconds :type "Float (single-precision)"))
  (bind (_returnvalue_x _returnvalue_y _returnvalue_z) (`KismetMathLibrary.BreakVector` (`SceneComponent.K2_GetComponentLocation` (`self.truck`))))
  (`SceneComponent.K2_AddWorldOffset` (`self.truck`) (`KismetMathLibrary.MakeVector` 0.0 (* DeltaSeconds (`self.moving`) (`self.multiplier`))) false false)
  (if (> _returnvalue_y 5000.0)
    (`SceneComponent.K2_SetWorldLocation` (`self.truck`) (`KismetMathLibrary.MakeVector` _returnvalue_x -5000.0 _returnvalue_z) false false)))

(fn `UserConstructionScript`)