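; Railway warning light actor that flashes two lights and sounds a warning as its assigned train approaches.
; Tick selects Train1 or Train2 by which reference is unset and checks the train's Y position against a threshold.
; In range, a Delay-driven FlipFlop alternates the lights, and the Warning plays once if the light is within an X window around the Player camera.
; Out of range, both lights hide and the warning flags reset.
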(event `self.ReceiveBeginPlay`
  (`SceneComponent.SetVisibility` (`self.light`) false false)
  (`SceneComponent.SetVisibility` (`self.light2`) false false))

(event `self.ReceiveTick`
  (params (DeltaSeconds :type "Float (single-precision)"))
  (bind _returnvalue_x (`KismetMathLibrary.BreakVector` (`SceneComponent.K2_GetComponentLocation` (`self.RL`))))
  (bind (_returnvalue_x_2 _returnvalue_y) (`KismetMathLibrary.BreakVector` (`SceneComponent.K2_GetComponentLocation` (`/Game/Blueprints/train2.train` (`self.train2`)))))
  (bind (_returnvalue_x_3 _returnvalue_y_2) (`KismetMathLibrary.BreakVector` (`SceneComponent.K2_GetComponentLocation` (`/Game/Blueprints/train.train` (`self.train1`)))))
  (if (== (`self.train1`) null)
    (if (> _returnvalue_y -500.0)
      (`KismetSystemLibrary.Delay` 0.25 :!label _label)
      (`/Engine/EditorBlueprintResources/StandardMacros.FlipFlop`
        (:`A`
          (`SceneComponent.SetVisibility` (`self.light`) false false)
          (`SceneComponent.SetVisibility` (`self.light2`) true false))
        (:`B`
          (`SceneComponent.SetVisibility` (`self.light`) true false)
          (`SceneComponent.SetVisibility` (`self.light2`) false false)))
      (bind _returnvalue (`GameplayStatics.GetActorOfClass` "/Game/Blueprints/Player.Player_C"))
      (if (`self.warningPlayed`)
        _
        (elif (`self.passed`)
          (set `self.passed` false)
          (else
            (bind _returnvalue_x_4 (`KismetMathLibrary.BreakVector` (`SceneComponent.K2_GetComponentLocation` (`/Game/Blueprints/Player.Camera` _returnvalue))))
            (if (and (> (- _returnvalue_x _returnvalue_x_4) -50.0) (< _returnvalue_x (+ _returnvalue_x_4 4500.0)))
              (`AudioComponent.Play` (`self.warning`) 0.0)
              (set `self.warningPlayed` true)))))
      (else
        (`SceneComponent.SetVisibility` (`self.light`) false false :!label _label_2)
        (`SceneComponent.SetVisibility` (`self.light2`) false false)
        (set `self.warningPlayed` false)
        (set `self.passed` true)))
    (elif (== (`self.train2`) null)
      (if (< _returnvalue_y_2 500.0)
        (goto _label)
        (else
          (goto _label_2))))))

(fn `UserConstructionScript`)