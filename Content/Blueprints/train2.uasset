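; Looping train actor that moves along the Y axis and plays a sound when it passes near the player.
; Tick offsets the Train by a frame-rate-independent speed and checks its position against a Y band and an X window around the Player's camera.
; A boolean latch triggers the audio once, resetting when the train is outside the Y band while inside the X window.
; Dropping below the despawn threshold teleports it back to the start and randomizes the next threshold.
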(event `self.ReceiveTick`
  (params (DeltaSeconds :type "Float (single-precision)"))
  (bind (_returnvalue_x _returnvalue_y _returnvalue_z) (`KismetMathLibrary.BreakVector` (`SceneComponent.K2_GetComponentLocation` (`self.train`))))
  (bind _returnvalue_x_2 (`KismetMathLibrary.BreakVector` (`SceneComponent.K2_GetComponentLocation` (`self.train`))))
  (bind (_returnvalue_x_3 _returnvalue_y_2) (`KismetMathLibrary.BreakVector` (`SceneComponent.K2_GetComponentLocation` (`self.train`))))
  (`SceneComponent.K2_AddWorldOffset` (`self.train`) (`KismetMathLibrary.MakeVector` 0.0 (* DeltaSeconds (`self.moving`))) false false)
  (bind _returnvalue (`GameplayStatics.GetActorOfClass` "/Game/Blueprints/Player.Player_C"))
  (bind _returnvalue_x_4 (`KismetMathLibrary.BreakVector` (`SceneComponent.K2_GetComponentLocation` (`/Game/Blueprints/Player.Camera` _returnvalue))))
  (if (and (> (- _returnvalue_x_2 _returnvalue_x_4) -50.0) (< _returnvalue_x_2 (+ _returnvalue_x_4 4500.0)))
    (if (and (< _returnvalue_y_2 2000.0) (> _returnvalue_y_2 -1000.0))
      (if (not (`self.trainSound`))
        (`AudioComponent.Play` (`self.Audio`) 0.0)
        (set `self.trainSound` true))
      (else
        (set `self.trainSound` false))))
  (if (< _returnvalue_y (`self.despawn`))
    (`SceneComponent.K2_SetWorldLocation` (`self.train`) (`KismetMathLibrary.MakeVector` _returnvalue_x 15000.0 _returnvalue_z) false false)
    (set `self.despawn` (`KismetMathLibrary.RandomFloatInRange` -15000.0 -30000.0))))

(fn `UserConstructionScript`)