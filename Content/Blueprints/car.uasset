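; Crossy Road-style car obstacle that picks one of three weighted random meshes on BeginPlay and drives along world Y.
; Each Tick moves it by delta time, Moving and Multiplier, then compares its X to the Player camera's.
; Within that window it rarely plays its audio at random.
; The wrap from Y above 5000 back to -5000 is checked only outside the window or after that audio roll succeeds.
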(event `self.ReceiveBeginPlay`
  (`StaticMeshComponent.SetStaticMesh` (`self.car`) (select `int` (`KismetMathLibrary.RandomIntegerInRange` 0 9) :`0` "/Game/Assets/car1/crossy_road_car_1.crossy_road_car_1" :`1` "/Game/Assets/car1/crossy_road_car_1.crossy_road_car_1" :`2` "/Game/Assets/car1/crossy_road_car_1.crossy_road_car_1" :`3` "/Game/Assets/car1/crossy_road_car_1.crossy_road_car_1" :`4` "/Game/Assets/car1/crossy_road_car_1.crossy_road_car_1" :`5` "/Game/Assets/car2/crossy_road_car_2.crossy_road_car_2" :`6` "/Game/Assets/car2/crossy_road_car_2.crossy_road_car_2" :`7` "/Game/Assets/car2/crossy_road_car_2.crossy_road_car_2" :`8` "/Game/Assets/car2/crossy_road_car_2.crossy_road_car_2" :`9` "/Game/Assets/car3/crossy_road_car_4.crossy_road_car_4" :!type "StaticMesh Object Reference")))

(event `self.ReceiveTick`
  (params (DeltaSeconds :type "Float (single-precision)"))
  (bind (_returnvalue_x _returnvalue_y _returnvalue_z) (`KismetMathLibrary.BreakVector` (`SceneComponent.K2_GetComponentLocation` (`self.car`))))
  (bind _returnvalue_x_2 (`KismetMathLibrary.BreakVector` (`SceneComponent.K2_GetComponentLocation` (`self.car`))))
  (`SceneComponent.K2_AddWorldOffset` (`self.car`) (`KismetMathLibrary.MakeVector` 0.0 (* DeltaSeconds (`self.moving`) (`self.multiplier`))) false false)
  (bind _returnvalue (`GameplayStatics.GetActorOfClass` "/Game/Blueprints/Player.Player_C"))
  (bind _returnvalue_x_3 (`KismetMathLibrary.BreakVector` (`SceneComponent.K2_GetComponentLocation` (`/Game/Blueprints/Player.Camera` _returnvalue))))
  (if (and (> (- _returnvalue_x_2 _returnvalue_x_3) -50.0) (< _returnvalue_x_2 (+ _returnvalue_x_3 4500.0)))
    (if (== (`KismetMathLibrary.RandomIntegerInRange` 0 2499) 0)
      (`AudioComponent.Play` (`self.Audio`) 0.0)
      (if (> _returnvalue_y 5000.0) :!label _label
        (`SceneComponent.K2_SetWorldLocation` (`self.car`) (`KismetMathLibrary.MakeVector` _returnvalue_x -5000.0 _returnvalue_z) false false)))
    (else
      (goto _label))))

(fn `UserConstructionScript`)